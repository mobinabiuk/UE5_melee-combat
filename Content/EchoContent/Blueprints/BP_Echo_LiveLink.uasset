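; BP_Echo_LiveLink is the Echo character Blueprint, named for Live Link use, that configures the character's body and hair at construction.
; The construction script fires ProxyConstruct, which lets the Body animate in the editor.
; A UseGroomAssets flag then selects groom hair and eyebrows with their bindings, or a skeletal mesh for the hair.
; BeginPlay is empty, so the Blueprint adds no runtime logic.
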(event `ProxyConstruct`
  (`SkeletalMeshComponent.SetUpdateAnimationInEditor` (`self.Body`) true))

(event `self.ReceiveBeginPlay`)

(fn `UserConstructionScript`
  (`self.ProxyConstruct`)
  (`|ExecutionSequence`
    (:`then_0`
      ;[1 1 1] Hair
      (if (`self.useGroomAssets`)
        (`GroomComponent.SetGroomAsset` (`self.HairGroom`) "/Game/EchoContent/Characters/Echo/Hair/Hair_S_UpdoBuns.Hair_S_UpdoBuns")
        (`GroomComponent.SetBindingAsset` (`self.HairGroom`) "/Game/EchoContent/Characters/Echo/Hair/Hair_S_UpdoBuns_Echo_M3D_LOD0_Binding.Hair_S_UpdoBuns_Echo_M3D_LOD0_Binding")
        (`GroomComponent.SetGroomAsset` (`self.EyebrowsGroom`) "/Game/EchoContent/Characters/Echo/Hair/Eyebrows_L_Echo.Eyebrows_L_Echo")
        (`GroomComponent.SetBindingAsset` (`self.EyebrowsGroom`) "/Game/EchoContent/Characters/Echo/Hair/Eyebrows_L_Echo_Echo_M3D_LOD0_Binding.Eyebrows_L_Echo_Echo_M3D_LOD0_Binding")
        (else
          (`SkinnedMeshComponent.SetSkinnedAssetAndUpdate` (`self.HairMesh`) "/Game/EchoContent/Characters/Echo/Meshes/Echo_Hair.Echo_Hair" true))))))